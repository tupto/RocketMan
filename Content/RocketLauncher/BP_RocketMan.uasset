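; First-person Rocket Man character Blueprint that adds audio, animation and aim feedback for a rocket launcher.
; Firing plays a launch sound and a shoot montage on the first-person rig.
; Falling or flying spawns an attached air whoosh whose volume and pitch Tick scales with speed above a threshold, until landing destroys it.
; Tick also moves a static mesh to the camera trace's impact point, alongside debug prints.
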(event `self.OnFire`
  ;[1 1 1] Shoot Sound
  (`GameplayStatics.SpawnSoundAtLocation` "/Game/RocketLauncher/SFX/LaunchCue.LaunchCue" (`self.K2_GetActorLocation`) (struct) 1.0 1.0 0.0 "/Game/RocketLauncher/SFX/SFXAttenuation.SFXAttenuation" null)
  (`AnimInstance.Montage_Play` (`SkeletalMeshComponent.GetAnimInstance` (`self.FPSRig`)) "/Game/RocketLauncher/FPSRig/FPSRig_Shoot_Montage.FPSRig_Shoot_Montage" 1.0 "MontageLength" 0.0 true))

(event `self.K2_OnStartCrouch`
  (params (HalfHeightAdjust :type "Float (single-precision)") (ScaledHalfHeightAdjust :type "Float (single-precision)"))
  (`KismetSystemLibrary.PrintString` "crouched"))

(event `self.K2_OnEndCrouch`
  (params (HalfHeightAdjust :type "Float (single-precision)") (ScaledHalfHeightAdjust :type "Float (single-precision)"))
  (`KismetSystemLibrary.PrintString` "uncrouched"))

(event `self.ReceiveBeginPlay`)

(event `self.OnLanded`
  (params (Hit :type "HitResult Structure (by ref)"))
  (bind _whooshcomponent (`self.WhooshComponent`))
  ;[1 1 1] Stop Whoosh On Land
  (`KismetSystemLibrary.PrintText` "Landed")
  (`/Engine/EditorBlueprintResources/StandardMacros.IsValid` _whooshcomponent
    (:`Is Valid`
      (`AudioComponent.SetPaused` _whooshcomponent true)
      (`ActorComponent.K2_DestroyComponent` _whooshcomponent))))

(event `self.K2_OnMovementModeChanged`
  (params (PrevMovementMode :type "EMovementMode Enum" :default "MOVE_None") (NewMovementMode :type "EMovementMode Enum" :default "MOVE_None") (PrevCustomMode :type Byte) (NewCustomMode :type Byte))
  (bind _charactermovement (`self.CharacterMovement`))
  (bind _returnvalue (/ (`KismetMathLibrary.FMax` (- (`KismetMathLibrary.VSize` (`self.GetVelocity`)) 800.0)) 2000.0))
  ;[1 1 1] Create Whoosh Sound
  (if (or (`NavMovementComponent.IsFlying` _charactermovement) (`NavMovementComponent.IsFalling` _charactermovement))
    (bind _returnvalue_2 (`GameplayStatics.SpawnSoundAttached` "/Game/RocketLauncher/SFX/AirWhistleCue.AirWhistleCue" (`self.FPSRig`) "None" (0.0 0.0 0.0) (struct) "KeepRelativeOffset" false (`KismetMathLibrary.Lerp` 0.0 0.2 _returnvalue) (`KismetMathLibrary.Lerp` 0.6 1.2 _returnvalue) 0.0 "/Game/RocketLauncher/SFX/SFXAttenuation.SFXAttenuation" null false))
    (set `self.WhooshComponent` _returnvalue_2)))

(event `self.ReceiveTick`
  (params (DeltaSeconds :type "Float (single-precision)"))
  (bind _fpscameracomponent (`self.FPSCameraComponent`))
  (bind _whooshcomponent (`self.WhooshComponent`))
  (bind _returnvalue (`SceneComponent.K2_GetComponentLocation` _fpscameracomponent))
  (bind _returnvalue_2 (/ (`KismetMathLibrary.FMax` (- (`KismetMathLibrary.VSize` (`self.GetVelocity`)) 800.0)) 2000.0))
  ;[1 1 1] Tick - Update Air Whoosh params
  (`KismetSystemLibrary.PrintString` (`KismetStringLibrary.Conv_DoubleToString` (`KismetMathLibrary.VSize` (`self.GetVelocity`))) true false (struct :`G` 0.66 :`B` 1.0 :`A` 1.0) 0.01)
  (bind _outhit (`KismetSystemLibrary.LineTraceSingle` _returnvalue (+ _returnvalue (* (`KismetMathLibrary.GetForwardVector` (`SceneComponent.K2_GetComponentRotation` _fpscameracomponent)) 10000.0)) "TraceTypeQuery1" true))
  (bind (_bblockinghit _binitialoverlap _time _distance _location _impactpoint) (`GameplayStatics.BreakHitResult` _outhit))
  (`SceneComponent.K2_SetWorldLocation` (`self.StaticMesh`) _impactpoint false false)
  (`KismetSystemLibrary.PrintString` (`KismetStringLibrary.Conv_VectorToString` _impactpoint) true true (struct :`G` 0.66 :`B` 1.0 :`A` 1.0) 0.01)
  (`/Engine/EditorBlueprintResources/StandardMacros.IsValid` _whooshcomponent
    (:`Is Valid`
      (`AudioComponent.SetVolumeMultiplier` _whooshcomponent (`KismetMathLibrary.Lerp` 0.0 0.2 _returnvalue_2))
      (`AudioComponent.SetPitchMultiplier` _whooshcomponent (`KismetMathLibrary.Lerp` 0.6 1.2 _returnvalue_2)))))

(fn `UserConstructionScript`)